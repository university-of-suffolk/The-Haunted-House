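; BP_Door is a double door with front and back panel pairs that slides open when the player enters its collision box while TargetHit is true.
; A timeline lerps the panels sideways, with a one-time creak sound and removal of the trigger box, then reverses after a delay, so it opens only once.
; TargetHit is never set here; projectile overlap and damage events only print debug text.
; The construction script assigns the panel meshes.
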(event `self.CollisionBox.OnComponentBeginOverlap`
  (params (OverlappedComponent :type "PrimitiveComponent Object Reference") (OtherActor :type "Actor Object Reference") (OtherComp :type "PrimitiveComponent Object Reference") (OtherBodyIndex :type Integer) (bFromSweep :type Boolean) (SweepResult :type "HitResult Structure (by ref)"))
  (if (== OtherActor (`GameplayStatics.GetPlayerCharacter` 0))
    (if (`self.TargetHit`)
      (bind (_direction _doortrack) (`Timeline|Timeline` :!label _label)
        (:`Update`
          (`|ExecutionSequence`
            (:`then_0`
              (`SceneComponent.K2_SetRelativeLocation` (`self.Door_Front_L`) (`KismetMathLibrary.MakeVector` (`KismetMathLibrary.Lerp` 0.0 -100.0 _doortrack)) false false)
              (`SceneComponent.K2_SetRelativeLocation` (`self.Door_Back_R`) (`KismetMathLibrary.MakeVector` (`KismetMathLibrary.Lerp` 0.0 -100.0 _doortrack)) false false))
            (:`then_1`
              (`SceneComponent.K2_SetRelativeLocation` (`self.Door_Front_R`) (`KismetMathLibrary.MakeVector` (`KismetMathLibrary.Lerp` 0.0 100.0 _doortrack)) false false)
              (`SceneComponent.K2_SetRelativeLocation` (`self.Door_Back_L`) (`KismetMathLibrary.MakeVector` (`KismetMathLibrary.Lerp` 0.0 100.0 _doortrack)) false false)))
          (`/Engine/EditorBlueprintResources/StandardMacros.DoOnce` false
            (:`Completed`
              (`GameplayStatics.PlaySoundAtLocation` "/Game/HorrorGameSounds/waves/CreakingDoor1.CreakingDoor1" (`self.K2_GetActorLocation`) (struct) 1.0 1.0 0.0 "/Game/TeamContent/Sounds/Attenuation_Sounds/SA_TargetHit.SA_TargetHit" null null null)
              (`ActorComponent.K2_DestroyComponent` (`self.CollisionBox`))
              (`KismetSystemLibrary.Delay` 3.0)
              (goto _label :!via `Reverse`))))))))

(event `self.Target.OnComponentBeginOverlap`
  (params (OverlappedComponent :type "PrimitiveComponent Object Reference") (OtherActor :type "Actor Object Reference") (OtherComp :type "PrimitiveComponent Object Reference") (OtherBodyIndex :type Integer) (bFromSweep :type Boolean) (SweepResult :type "HitResult Structure (by ref)"))
  (cast `/Game/FirstPerson/Blueprints/BP_FirstPersonProjectile` OtherActor)
  (`KismetSystemLibrary.PrintString` "1"))

(event `self.ReceiveAnyDamage`
  (params (Damage :type "Float (single-precision)") (DamageType :type "DamageType Object Reference") (InstigatedBy :type "Controller Object Reference") (DamageCauser :type "Actor Object Reference"))
  (`KismetSystemLibrary.PrintString` "2"))

(fn `UserConstructionScript`
  (bind _frontdoor (`self.FrontDoor`))
  (bind _backdoor (`self.BackDoor`))
  (`|ExecutionSequence`
    (:`then_0`
      (`StaticMeshComponent.SetStaticMesh` (`self.Door_Front_L`) _frontdoor)
      (`StaticMeshComponent.SetStaticMesh` (`self.Door_Front_R`) _frontdoor))
    (:`then_1`
      (`StaticMeshComponent.SetStaticMesh` (`self.Door_Back_L`) _backdoor)
      (`StaticMeshComponent.SetStaticMesh` (`self.Door_Back_R`) _backdoor))))