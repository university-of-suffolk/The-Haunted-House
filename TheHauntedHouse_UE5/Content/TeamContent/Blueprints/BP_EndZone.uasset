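; BP_EndZone is a trigger volume that ends the level when the first-person character overlaps its collision box.
; It shows the RestartLevel widget, switches input to UI only with a visible mouse cursor, then copies the character's run time and distance traveled into its own variables.
; The copy runs after the widget is created and added to the viewport.
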(event `self.CollisionBox.OnComponentBeginOverlap`
  (params (OverlappedComponent :type "PrimitiveComponent Object Reference") (OtherActor :type "Actor Object Reference") (OtherComp :type "PrimitiveComponent Object Reference") (OtherBodyIndex :type Integer) (bFromSweep :type Boolean) (SweepResult :type "HitResult Structure (by ref)"))
  (bind _returnvalue (`GameplayStatics.GetPlayerController` 0))
  (bind _asbp_first_person_character (cast `/Game/FirstPerson/Blueprints/BP_FirstPersonCharacter` OtherActor))
  (`|ExecutionSequence`
    (:`then_0`
      (bind _returnvalue_2 (`|CreateWidget` "/Game/TeamContent/UI/RestartLevel.RestartLevel_C"))
      (`UserWidget.AddToViewport` _returnvalue_2 0)
      (`WidgetBlueprintLibrary.SetInputMode_UIOnlyEx` _returnvalue _returnvalue_2)
      (set `PlayerController.bShowMouseCursor` true _returnvalue))
    (:`then_1`
      ;[1 1 1] TimeRef
      (set `self.MinRef` (`/Game/FirstPerson/Blueprints/BP_FirstPersonCharacter.TimeInMin` _asbp_first_person_character))
      (set `self.SecRef` (`/Game/FirstPerson/Blueprints/BP_FirstPersonCharacter.TimeInSeconds` _asbp_first_person_character))
      (set `self.MilisecRef` (`/Game/FirstPerson/Blueprints/BP_FirstPersonCharacter.TimeInMiliSec` _asbp_first_person_character))
      (set `self.DistanceRef` (`/Game/FirstPerson/Blueprints/BP_FirstPersonCharacter.DistanceTraveled` _asbp_first_person_character)))))

(fn `UserConstructionScript`)