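; BP_Target is a shootable target actor that awards points to the player when destroyed.
; BeginPlay caches the first player's BP_FirstPersonCharacter.
; AnyDamage subtracts damage from TargetHealth, playing a hit sound at the TargetMonsterMesh location while health remains.
; At zero health or below, it gives TargetPoints to that cached character, plays an explosion sound and destroys itself, regardless of who dealt the damage.
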(event `self.ReceiveBeginPlay`
  (bind _asbp_first_person_character (cast `/Game/FirstPerson/Blueprints/BP_FirstPersonCharacter` (`GameplayStatics.GetPlayerCharacter` 0)))
  (set `self.FirstPersonCharacter` _asbp_first_person_character))

(event `self.ReceiveAnyDamage`
  (params (Damage :type "Float (single-precision)") (DamageType :type "DamageType Object Reference") (InstigatedBy :type "Controller Object Reference") (DamageCauser :type "Actor Object Reference"))
  (bind _output_get (set `self.TargetHealth` (- (`self.TargetHealth`) Damage)))
  (if (<= _output_get 0.0)
    (`/Game/FirstPerson/Blueprints/BP_FirstPersonCharacter.GivePoints` (`self.FirstPersonCharacter`) (`self.TargetPoints`))
    (`GameplayStatics.PlaySoundAtLocation` "/Game/StarterContent/Audio/Explosion01.Explosion01" (`SceneComponent.K2_GetComponentLocation` (`self.TargetMonsterMesh`)) (struct) 1.0 1.0 0.0 null null null null)
    (`self.K2_DestroyActor`)
    (else
      (`GameplayStatics.PlaySoundAtLocation` "/Engine/EditorSounds/Notifications/CompileSuccess.CompileSuccess" (`SceneComponent.K2_GetComponentLocation` (`self.TargetMonsterMesh`)) (struct) 1.0 1.0 0.0 null null null null))))

(fn `UserConstructionScript`)