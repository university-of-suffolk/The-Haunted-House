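; BP_Pumkin is a damageable pumpkin target that awards points to the first-person player when destroyed.
; It caches the player character on BeginPlay and subtracts incoming damage from its health.
; At zero health it gives the player its points, plays hit and bone-cracking sounds, spawns a points display at the mesh, increments the player's hit count and destroys itself.
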(event `self.ReceiveBeginPlay`
  (bind _asbp_first_person_character (cast `/Game/FirstPerson/Blueprints/BP_FirstPersonCharacter` (`GameplayStatics.GetPlayerCharacter` 0)))
  (set `self.FirstPersonCharacter` _asbp_first_person_character))

(event `self.ReceiveAnyDamage`
  (params (Damage :type "Float (single-precision)") (DamageType :type "DamageType Object Reference") (InstigatedBy :type "Controller Object Reference") (DamageCauser :type "Actor Object Reference"))
  (bind _firstpersoncharacter (`self.FirstPersonCharacter`))
  (bind _output_get (set `self.TargetHealth` (- (`self.TargetHealth`) Damage)))
  (if (<= _output_get 0.0)
    (`/Game/FirstPerson/Blueprints/BP_FirstPersonCharacter.GivePoints` (`self.FirstPersonCharacter`) (`self.TargetPoints`))
    (`GameplayStatics.PlaySoundAtLocation` "/Game/TeamContent/Sounds/Sound_Cues/SC_TargetHit.SC_TargetHit" (`SceneComponent.K2_GetComponentLocation` (`self.ExplosiveMesh`)) (struct) 1.0 1.0 0.0 null null null null)
    (`GameplayStatics.PlaySoundAtLocation` "/Game/HorrorGameSounds/waves/BoneCracking4.BoneCracking4" (`SceneComponent.K2_GetComponentLocation` (`self.ExplosiveMesh`)) (struct) 1.0 1.0 0.0 null null null null)
    (`|SpawnActorFromClass` "/Game/TeamContent/Blueprints/BP_PointsDisplay.BP_PointsDisplay_C" (`SceneComponent.K2_GetComponentToWorld` (`self.ExplosiveMesh`)) "Undefined" "OverrideRootScale" null (`self.TargetPoints`) null)
    (bind _result (`/Engine/EditorBlueprintResources/StandardMacros.IncrementInt` (`/Game/FirstPerson/Blueprints/BP_FirstPersonCharacter.TargetsHit` _firstpersoncharacter))
      (:`  `
        (set `/Game/FirstPerson/Blueprints/BP_FirstPersonCharacter.TargetsHit` _result _firstpersoncharacter)
        (`self.K2_DestroyActor`)))))

(fn `UserConstructionScript`)