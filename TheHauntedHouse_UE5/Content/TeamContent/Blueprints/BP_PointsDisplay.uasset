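; BP_PointsDisplay is a short-lived actor that shows a points amount as a floating popup in the world.
; On BeginPlay it copies its Points value into the W_PointsDisplay widget held by its widget component.
; The Move timeline then lerps the actor from its spawn location to a fixed raised, diagonal offset and destroys it when finished.
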(event `self.ReceiveBeginPlay`
  (bind _asw_points_display (cast `/Game/TeamContent/UI/W_PointsDisplay` (`WidgetComponent.GetWidget` (`self.Widget`))))
  (set `/Game/TeamContent/UI/W_PointsDisplay.PointsAmount` (`self.Points`) _asw_points_display)
  (bind _output_get (set `self.StartLocation` (`self.K2_GetActorLocation`)))
  (set `self.EndLocation` (+ _output_get (-25.0 -25.0 50.0)))
  (bind (_direction _move_track) (`Timeline|Move`)
    (:`Update`
      (`self.K2_SetActorLocation` (`KismetMathLibrary.VLerp` (`self.StartLocation`) (`self.EndLocation`) _move_track)))
    (:`Finished`
      (`self.K2_DestroyActor`))))

(fn `UserConstructionScript`)