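; BP_Trap_Explosive is a destructible explosive trap that can be shot for points or hurts the player on contact.
; Incoming damage lowers TargetHealth; at zero it awards TargetPoints to the cached first-person character and plays a hit sound.
; Player overlap with DamageSphere calls DamagePlayer instead.
; Both paths share the explosion sound, points display spawn and self-destruction, so the display appears even when no points are awarded.
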(event `self.ReceiveBeginPlay`
  (bind _asbp_first_person_character (cast `/Game/FirstPerson/Blueprints/BP_FirstPersonCharacter` (`GameplayStatics.GetPlayerCharacter` 0)))
  (set `self.FirstPersonCharacter` _asbp_first_person_character))

(event `self.ReceiveAnyDamage`
  (params (Damage :type "Float (single-precision)") (DamageType :type "DamageType Object Reference") (InstigatedBy :type "Controller Object Reference") (DamageCauser :type "Actor Object Reference"))
  (bind _output_get (set `self.TargetHealth` (- (`self.TargetHealth`) Damage)))
  (if (<= _output_get 0.0)
    (`/Game/FirstPerson/Blueprints/BP_FirstPersonCharacter.GivePoints` (`self.FirstPersonCharacter`) (`self.TargetPoints`))
    (`GameplayStatics.PlaySoundAtLocation` "/Game/TeamContent/Sounds/Sound_Cues/SC_TargetHit.SC_TargetHit" (`SceneComponent.K2_GetComponentLocation` (`self.ExplosiveMesh`)) (struct) 1.0 1.0 0.0 null null null null)
    (`GameplayStatics.PlaySoundAtLocation` "/Game/StarterContent/Audio/Explosion01.Explosion01" (`SceneComponent.K2_GetComponentLocation` (`self.ExplosiveMesh`)) (struct) 1.0 1.0 0.0 null null null null :!label _label)
    (`|SpawnActorFromClass` "/Game/TeamContent/Blueprints/BP_PointsDisplay.BP_PointsDisplay_C" (`SceneComponent.K2_GetComponentToWorld` (`self.ExplosiveMesh`)) "Undefined" "OverrideRootScale" null (`self.TargetPoints`) null)
    (`self.K2_DestroyActor`)))

(event `self.DamageSphere.OnComponentBeginOverlap`
  (params (OverlappedComponent :type "PrimitiveComponent Object Reference") (OtherActor :type "Actor Object Reference") (OtherComp :type "PrimitiveComponent Object Reference") (OtherBodyIndex :type Integer) (bFromSweep :type Boolean) (SweepResult :type "HitResult Structure (by ref)"))
  (if (== OtherActor (`GameplayStatics.GetPlayerCharacter` 0))
    (`/Game/FirstPerson/Blueprints/BP_FirstPersonCharacter.DamagePlayer` (`self.FirstPersonCharacter`))
    (goto _label)))

(fn `UserConstructionScript`)