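; BP_FriendlyTarget is a shootable target that opens and activates the first time the first-person character enters its detection sphere.
; Damage drains its health; at zero while active, it closes, awards points and increments the player's targets-hit count.
; The hit also plays a sound and spawns a points display, then deactivates the target.
; The construction script snaps the monster mesh to a skeletal base socket.
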(event `self.ReceiveBeginPlay`
  (bind _asbp_first_person_character (cast `/Game/FirstPerson/Blueprints/BP_FirstPersonCharacter` (`GameplayStatics.GetPlayerCharacter` 0)))
  (set `self.FirstPersonCharacter` _asbp_first_person_character))

(event `self.ReceiveAnyDamage`
  (params (Damage :type "Float (single-precision)") (DamageType :type "DamageType Object Reference") (InstigatedBy :type "Controller Object Reference") (DamageCauser :type "Actor Object Reference"))
  (bind _output_get (set `self.TargetHealth` (- (`self.TargetHealth`) Damage)))
  (if (and (<= _output_get 0.0) (`self.IsActive?`))
    (`SkeletalMeshComponent.PlayAnimation` (`self.SK_TargetBase`) "/Game/TeamContent/Models/Animations/AnimSeq_Target_Close.AnimSeq_Target_Close" false)
    (`/Game/FirstPerson/Blueprints/BP_FirstPersonCharacter.GivePoints` (`self.FirstPersonCharacter`) (`self.TargetPoints`))
    (set `/Game/FirstPerson/Blueprints/BP_FirstPersonCharacter.TargetsHit` (+ (`/Game/FirstPerson/Blueprints/BP_FirstPersonCharacter.TargetsHit` (`self.FirstPersonCharacter`)) 1) (`self.FirstPersonCharacter`)) ; Keep Track of Targets Hit by the Player
    (`GameplayStatics.PlaySoundAtLocation` "/Game/TeamContent/Sounds/Sound_Cues/SC_TargetHit.SC_TargetHit" (`SceneComponent.K2_GetComponentLocation` (`self.TargetMonsterMesh`)) (struct) 1.0 1.0 0.0 null null null null)
    (`|SpawnActorFromClass` "/Game/TeamContent/Blueprints/BP_PointsDisplay.BP_PointsDisplay_C" (`SceneComponent.K2_GetComponentToWorld` (`self.MonsterImagePlane`)) "Undefined" "OverrideRootScale" null (`self.TargetPoints`) null)
    (set `self.IsActive?` false)))

(event `self.DetectPlayerSphere.OnComponentBeginOverlap`
  (params (OverlappedComponent :type "PrimitiveComponent Object Reference") (OtherActor :type "Actor Object Reference") (OtherComp :type "PrimitiveComponent Object Reference") (OtherBodyIndex :type Integer) (bFromSweep :type Boolean) (SweepResult :type "HitResult Structure (by ref)"))
  (cast `/Game/FirstPerson/Blueprints/BP_FirstPersonCharacter` OtherActor)
  (`/Engine/EditorBlueprintResources/StandardMacros.DoOnce` false
    (:`Completed`
      (`SkeletalMeshComponent.PlayAnimation` (`self.SK_TargetBase`) "/Game/TeamContent/Models/Animations/AnimSeq_Target_Open.AnimSeq_Target_Open" false)
      (set `self.IsActive?` true))))

(fn `UserConstructionScript`
  (`SceneComponent.K2_AttachToComponent` (`self.TargetMonsterMesh`) (`self.SK_TargetBase`) "Monster_pointSocket" "SnapToTarget" "SnapToTarget" "KeepWorld" true))