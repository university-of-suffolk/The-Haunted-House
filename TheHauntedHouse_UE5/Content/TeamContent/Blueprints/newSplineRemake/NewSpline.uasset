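; Spline actor, apparently an unfinished remake, meant to lock the first-person character onto a spline path.
; Overlaps on its begin and end triggers call BeginSpline or EndSpline according to the sign of the player's Y velocity.
; Both events, BeginPlay and Tick are empty; the logic for caching the player, setting spline state and snapping the capsule to the closest spline point is disconnected and never runs.
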(event `self.ReceiveBeginPlay`
  ;[1 1 1] Spline
)

(event `self.ReceiveTick`
  (params (DeltaSeconds :type "Float (single-precision)")))

(event `BeginSpline`
  ;[1 1 1] beign and end spline
)

(event `EndSpline`
  ;[1 1 1] beign and end spline
)

(event `self.SplineBegin.OnComponentBeginOverlap`
  (params (OverlappedComponent :type "PrimitiveComponent Object Reference") (OtherActor :type "Actor Object Reference") (OtherComp :type "PrimitiveComponent Object Reference") (OtherBodyIndex :type Integer) (bFromSweep :type Boolean) (SweepResult :type "HitResult Structure (by ref)"))
  (bind _fpcref (`self.FPCRef`))
  (bind (_velocity_x _velocity_y) (`KismetMathLibrary.BreakVector` (`MovementComponent.Velocity` (`Character.CharacterMovement` _fpcref))))
  (if (== OtherActor _fpcref)
    (if (< _velocity_y 0.0)
      (`self.BeginSpline`)
      (else
        (`self.EndSpline`)))))

(event `self.SplineEnd.OnComponentBeginOverlap`
  (params (OverlappedComponent :type "PrimitiveComponent Object Reference") (OtherActor :type "Actor Object Reference") (OtherComp :type "PrimitiveComponent Object Reference") (OtherBodyIndex :type Integer) (bFromSweep :type Boolean) (SweepResult :type "HitResult Structure (by ref)"))
  (bind _fpcref (`self.FPCRef`))
  (bind (_velocity_x _velocity_y) (`KismetMathLibrary.BreakVector` (`MovementComponent.Velocity` (`Character.CharacterMovement` _fpcref))))
  (if (== OtherActor _fpcref)
    (if (< _velocity_y 0.0)
      (`self.BeginSpline`)
      (else
        (`self.EndSpline`)))))

(fn `UserConstructionScript`)