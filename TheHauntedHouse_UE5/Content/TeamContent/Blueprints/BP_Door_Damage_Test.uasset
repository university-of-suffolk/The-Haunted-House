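; Sliding door actor that opens once its linked TargetForDoor has been hit.
; BeginPlay grabs a single TargetForDoor via GetActorOfClass, and Tick polls its HasBeenHit flag to play a timeline.
; The timeline slides four front and back panels in opposing X directions, with a DoOnce creak sound at the door.
; The construction script assigns the FrontDoor and BackDoor meshes to the panels.
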(event `self.ReceiveTick`
  (params (DeltaSeconds :type "Float (single-precision)"))
  (if (`/Game/TeamContent/Blueprints/TargetForDoor.HasBeenHit` (`self.TargetForDoorRef`))
    (bind (_direction _doortrack) (`Timeline|Timeline`)
      (:`Update`
        (`|ExecutionSequence`
          (:`then_0`
            (`SceneComponent.K2_SetRelativeLocation` (`self.Door_Front_L`) (`KismetMathLibrary.MakeVector` (`KismetMathLibrary.Lerp` 0.0 -100.0 _doortrack)) false false)
            (`SceneComponent.K2_SetRelativeLocation` (`self.Door_Back_R`) (`KismetMathLibrary.MakeVector` (`KismetMathLibrary.Lerp` 0.0 -100.0 _doortrack)) false false))
          (:`then_1`
            (`SceneComponent.K2_SetRelativeLocation` (`self.Door_Front_R`) (`KismetMathLibrary.MakeVector` (`KismetMathLibrary.Lerp` 0.0 100.0 _doortrack)) false false)
            (`SceneComponent.K2_SetRelativeLocation` (`self.Door_Back_L`) (`KismetMathLibrary.MakeVector` (`KismetMathLibrary.Lerp` 0.0 100.0 _doortrack)) false false)))
        (`/Engine/EditorBlueprintResources/StandardMacros.DoOnce` false
          (:`Completed`
            (`GameplayStatics.PlaySoundAtLocation` "/Game/HorrorGameSounds/waves/CreakingDoor1.CreakingDoor1" (`self.K2_GetActorLocation`) (struct) 1.0 1.0 0.0 "/Game/TeamContent/Sounds/Attenuation_Sounds/SA_TargetHit.SA_TargetHit" null null null)))))))

(event `self.ReceiveBeginPlay`
  (bind _returnvalue (`GameplayStatics.GetActorOfClass` "/Game/TeamContent/Blueprints/TargetForDoor.TargetForDoor_C"))
  (bind _astarget_for_door (cast `/Game/TeamContent/Blueprints/TargetForDoor` _returnvalue))
  (set `self.TargetForDoorRef` _astarget_for_door))

(fn `UserConstructionScript`
  (bind _frontdoor (`self.FrontDoor`))
  (bind _backdoor (`self.BackDoor`))
  (`|ExecutionSequence`
    (:`then_0`
      (`StaticMeshComponent.SetStaticMesh` (`self.Door_Front_L`) _frontdoor)
      (`StaticMeshComponent.SetStaticMesh` (`self.Door_Front_R`) _frontdoor))
    (:`then_1`
      (`StaticMeshComponent.SetStaticMesh` (`self.Door_Back_L`) _backdoor)
      (`StaticMeshComponent.SetStaticMesh` (`self.Door_Back_R`) _backdoor))))